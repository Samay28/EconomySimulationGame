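; BP_TutorialPawn runs the game's intro flow: a startup cinematic with music, then a tutorial video, then the MainWorld level.
; Fixed delays advance each stage, with no playback-finished events.
; Speech recognition listens for "skip", which jumps from the cinematic to the video widget, or from the video straight to MainWorld.
; The IsCinematicOpen flag tracks the stage and guards the timed transition after an early skip.
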(event `self.ReceiveBeginPlay`
  (add `SpeechRecognitionSubsystem.OnWordsSpoken` (subsystem `SpeechRecognitionSubsystem`) (delegate `TriggerSpeech`))
  (bind (_outactor _returnvalue) (`LevelSequencePlayer.CreateLevelSequencePlayer` "/Game/Cinematics/Sequences/StartupMovie/StartupMovieRoot.StartupMovieRoot"))
  (`MovieSceneSequencePlayer.Play` _returnvalue)
  (bind _returnvalue_2 (`GameplayStatics.SpawnSound2D` "/Game/RetroGameplayLoops/Cue/Loop_7_Cue.Loop_7_Cue" 1.0 1.0 0.0 null))
  (`AudioComponent.Play` _returnvalue_2 0.0)
  (`KismetSystemLibrary.Delay` 30.0)
  (if (`self.isCinematicOpen`)
    (`MovieSceneSequencePlayer.Stop` _returnvalue :!label _label)
    (bind _returnvalue_3 (`|CreateWidget` "/Game/Widgets/WBP_TutorialVideo.WBP_TutorialVideo_C" (`GameplayStatics.GetPlayerController` 0)))
    (`UserWidget.AddToViewport` _returnvalue_3 0)
    (set `self.isCinematicOpen` false)
    (`AudioComponent.Stop` _returnvalue_2)
    (`KismetSystemLibrary.Delay` 86.0)
    (`GameplayStatics.OpenLevel` "MainWorld")))

(event `TriggerSpeech`
  (params (Text :type "RecognisedPhrases Structure"))
  (bind _iscinematicopen (`self.isCinematicOpen`))
  (for _array_element (`.phrases` (break `RecognisedPhrases` Text))
    (bind _returnvalue (== _array_element "skip"))
    (if (and _returnvalue _iscinematicopen)
      (goto _label)
      (elif (and _returnvalue (not _iscinematicopen))
        (`GameplayStatics.OpenLevel` "MainWorld")))))

(fn `UserConstructionScript`)