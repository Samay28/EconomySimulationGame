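; GS_NewState is a manager Blueprint, apparently a Game State, that sets up the voice command vocabulary for a building and economy game.
; On BeginPlay it switches the Speech Recognition Subsystem into keyword mode with a fixed phrase list covering movement, construction, trading, menus and pausing.
; Each phrase carries its own match tolerance.
; It only registers the keywords and contains no handling of recognized phrases.
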(event `self.ReceiveBeginPlay`
  (`SpeechRecognitionSubsystem.EnableKeywordMode` (subsystem `SpeechRecognitionSubsystem`) (`|MakeArray` (make `RecognitionPhrase` "Move" "VE_8") (make `RecognitionPhrase` "Left" "VE_8") (make `RecognitionPhrase` "make house" "VE_7") (make `RecognitionPhrase` "Right" "VE_8") (make `RecognitionPhrase` "Back" "VE_8") (make `RecognitionPhrase` "Stop" "VE_8") (make `RecognitionPhrase` "make farm" "VE_7") (make `RecognitionPhrase` "start cutting" "VE_7") (make `RecognitionPhrase` "Pause Game" "VE_7") (make `RecognitionPhrase` "resume" "VE_7") (make `RecognitionPhrase` "economy" "VE_7") (make `RecognitionPhrase` "exit" "VE_7") (make `RecognitionPhrase` "ok" "VE_7") (make `RecognitionPhrase` "speech" "VE_7") (make `RecognitionPhrase` "buy land" "VE_7") (make `RecognitionPhrase` "make shop" "VE_7") (make `RecognitionPhrase` "sell" "VE_7") (make `RecognitionPhrase` "open shop" "VE_7") (make `RecognitionPhrase` "Forest" "VE_7") (make `RecognitionPhrase` "go home" "VE_7") (make `RecognitionPhrase` "items" "VE_7") (make `RecognitionPhrase` "first" "VE_7") (make `RecognitionPhrase` "second" "VE_7") (make `RecognitionPhrase` "third" "VE_7") (make `RecognitionPhrase` "make pond"))))

(fn `UserConstructionScript`)