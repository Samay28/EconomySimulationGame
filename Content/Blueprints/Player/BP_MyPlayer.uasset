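; BP_MyPlayer is the player Blueprint that turns spoken commands into movement, teleport and menu actions.
; BeginPlay binds TriggerSpeech to the speech recognition subsystem and shows the main UI.
; TriggerSpeech runs each recognized phrase through a chain of string comparisons, calling movement functions or opening pause, inventory and auto-travel widgets.
; Pausing also blocks movement through BP_GameManager, and "ok" closes the inventory only while it is open.
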(event `self.ReceiveBeginPlay`
  (add `SpeechRecognitionSubsystem.OnWordsSpoken` (subsystem `SpeechRecognitionSubsystem`) (delegate `TriggerSpeech`))
  (bind _returnvalue (`|CreateWidget` "/Game/Widgets/WBP_MainUI.WBP_MainUI_C"))
  (`UserWidget.AddToViewport` _returnvalue 0))

(event `TriggerSpeech`
  (params (Text :type "RecognisedPhrases Structure"))
  (for _array_element (`.phrases` (break `RecognisedPhrases` Text))
    (if (== _array_element "Move")
      (`self.MoveForward`)
      (elif (== _array_element "Left")
        (`self.MoveLeft`)
        (elif (== _array_element "right")
          (`self.MoveRight`)
          (elif (== _array_element "back")
            (`self.MoveBackward`)
            (elif (== _array_element "stop")
              (`self.StopMovement`)
              (elif (== _array_element "pause game")
                (bind _returnvalue (`|CreateWidget` "/Game/Widgets/WBP_MainUI.WBP_MainUI_C"))
                (`Widget.RemoveFromParent` _returnvalue)
                (bind _returnvalue_2 (`|CreateWidget` "/Game/Widgets/WBP_PauseGame.WBP_PauseGame_C"))
                (`UserWidget.AddToViewport` _returnvalue_2 0)
                (bind _returnvalue_3 (`GameplayStatics.GetActorOfClass` "/Game/Blueprints/Manager/BP_GameManager.BP_GameManager_C"))
                (set `GameManager.BlockPlayerMovement` true _returnvalue_3)
                (elif (== _array_element "Forest")
                  (`self.TeleportPlayer`)
                  (elif (== _array_element "go home")
                    (`self.SendBackPlayer`)
                    (elif (== _array_element "items")
                      (bind _returnvalue_4 (`|CreateWidget` "/Game/Widgets/WBP_SingleInventory.WBP_SingleInventory_C"))
                      (`UserWidget.AddToViewport` _returnvalue_4 0)
                      (set `self.IsInventoryOpen` true)
                      (elif (and (== _array_element "ok") (`self.IsInventoryOpen`))
                        (`Widget.RemoveFromParent` _returnvalue_4)
                        (set `self.IsInventoryOpen` false)
                        (elif (== _array_element "fast")
                          (bind _returnvalue_5 (`|CreateWidget` "/Game/Widgets/WBP_AutoTravel.WBP_AutoTravel_C"))
                          (`UserWidget.AddToViewport` _returnvalue_5 0))))))))))))))

(fn `UserConstructionScript`)