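; BP_Tree is a tree the player can cut down by voice command while standing in its overlap volume.
; Overlap by BP_MyPlayer on a cuttable tree shows a WBP_MainUI prompt and binds to SpeechRecognitionSubsystem.
; Hearing "start cutting" during contact calls StartCuttingTrees, plays a looping-until-stopped sound, and drives a progress bar from the CuttingTimer timeline.
; Leaving hides the prompt and disables the mesh's custom depth.
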(event `self.Overlaping.OnComponentBeginOverlap`
  (params (OverlappedComponent :type "PrimitiveComponent Object Reference") (OtherActor :type "Actor Object Reference") (OtherComp :type "PrimitiveComponent Object Reference") (OtherBodyIndex :type Integer) (bFromSweep :type Boolean) (SweepResult :type "HitResult Structure (by ref)"))
  (if (`self.CanBeCut`)
    (cast `/Game/Blueprints/Player/BP_MyPlayer` OtherActor)
    (set `self.HasContact` true)
    (bind _foundwidgets (`WidgetBlueprintLibrary.GetAllWidgetsOfClass` "/Game/Widgets/WBP_MainUI.WBP_MainUI_C"))
    (if (> (`KismetArrayLibrary.Array_Length` _foundwidgets) 0)
      (`Widget.SetVisibility` (`/Game/Widgets/WBP_MainUI.StartCuttingPrompt` (`|GetArrayItem` _foundwidgets)) "Visible")
      (add `SpeechRecognitionSubsystem.OnWordsSpoken` (subsystem `SpeechRecognitionSubsystem`) (delegate `TriggerSpeech`))
      (else
        (`KismetSystemLibrary.PrintString` "Hello")))))

(event `TriggerSpeech`
  (params (Text :type "RecognisedPhrases Structure"))
  (for _array_element (`.phrases` (break `RecognisedPhrases` Text))
    (if (== _array_element "start cutting")
      (if (`self.HasContact`)
        (`self.StartCuttingTrees`)
        (bind _returnvalue (`GameplayStatics.SpawnSound2D` "/Game/AUDIO/Tree/SC_TreeCutting.SC_TreeCutting" 1.0 1.0 0.0 null))
        (bind _output (`|GetArrayItem` (stale `self.Overlaping.OnComponentBeginOverlap` _foundwidgets)))
        (`Widget.SetVisibility` (`/Game/Widgets/WBP_MainUI.StartCuttingPrompt` _output) "Hidden")
        (bind _cuttingprogress (`/Game/Widgets/WBP_MainUI.CuttingProgress` _output))
        (`Widget.SetVisibility` _cuttingprogress "Visible")
        (bind (_direction _cuttingtrack) (`Timeline|CuttingTimer` :!via `PlayFromStart`)
          (:`Update`
            (`ProgressBar.SetPercent` _cuttingprogress _cuttingtrack))
          (:`Finished`
            (`ProgressBar.SetPercent` _cuttingprogress 0.0)
            (`Widget.SetVisibility` _cuttingprogress "Hidden")
            (`AudioComponent.Stop` _returnvalue)))))))

(event `self.Overlaping.OnComponentEndOverlap`
  (params (OverlappedComponent :type "PrimitiveComponent Object Reference") (OtherActor :type "Actor Object Reference") (OtherComp :type "PrimitiveComponent Object Reference") (OtherBodyIndex :type Integer))
  (cast `/Game/Blueprints/Player/BP_MyPlayer` OtherActor)
  (set `self.HasContact` false)
  (`PrimitiveComponent.SetRenderCustomDepth` (`self.TreeMesh`) false)
  (bind _foundwidgets (`WidgetBlueprintLibrary.GetAllWidgetsOfClass` "/Game/Widgets/WBP_MainUI.WBP_MainUI_C"))
  (`Widget.SetVisibility` (`/Game/Widgets/WBP_MainUI.StartCuttingPrompt` (`|GetArrayItem` _foundwidgets)) "Hidden"))

(fn `UserConstructionScript`)