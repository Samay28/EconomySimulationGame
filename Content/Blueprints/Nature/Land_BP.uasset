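; Land plot actor the player buys and develops by voice command into a house, farm, shop, pond or mine.
; Player overlap shows a prompt widget on unrented plots and binds speech recognition, whose phrases are gated by contact, rental and occupancy flags.
; "make shop" opens a choice widget and blocks movement through BP_GameManager, with most shop types gated by island value.
; Purchase and conversion results select success or error audio.
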(event `self.Overlap.OnComponentBeginOverlap`
  (params (OverlappedComponent :type "PrimitiveComponent Object Reference") (OtherActor :type "Actor Object Reference") (OtherComp :type "PrimitiveComponent Object Reference") (OtherBodyIndex :type Integer) (bFromSweep :type Boolean) (SweepResult :type "HitResult Structure (by ref)"))
  (if (`self.ActorHasTag` OtherActor "Player")
    (if (not (`self.bIsRented`))
      (`SceneComponent.SetVisibility` (`self.Widget`) true false))
    (set `self.IsContact` true)
    (add `SpeechRecognitionSubsystem.OnWordsSpoken` (subsystem `SpeechRecognitionSubsystem`) (delegate `TriggerSpeech`))))

(event `TriggerSpeech`
  (params (Text :type "RecognisedPhrases Structure"))
  (for _array_element (`.phrases` (break `RecognisedPhrases` Text))
    (if (`self.IsOccupied`)
      _
      (elif (and (== _array_element "Buy Land") (`self.IsContact`) (not (`self.bIsRented`)))
        (`SceneComponent.SetVisibility` (`self.Widget`) false false)
        (bind _returnvalue (`self.PurchaseLand`))
        (`self.PlaySetupAudio` _returnvalue)
        (elif (and (== _array_element "Make House") (`self.IsContact`) (`self.bIsRented`))
          (bind _returnvalue_2 (`self.ConvertToHouse`))
          (`self.PlaySetupAudio` _returnvalue_2)
          (elif (and (== _array_element "Make Farm") (`self.IsContact`) (`self.bIsRented`))
            (bind _returnvalue_3 (`self.ConvertToFarm`))
            (`self.PlaySetupAudio` _returnvalue_3)
            (elif (and (== _array_element "make shop") (`self.IsContact`) (`self.bIsRented`))
              (bind _returnvalue_4 (`|CreateWidget` "/Game/Widgets/WBP_ShopChoice.WBP_ShopChoice_C"))
              (`UserWidget.AddToViewport` _returnvalue_4 0)
              (set `self.IsShopChoiceOpen` true)
              (bind _returnvalue_5 (`GameplayStatics.GetActorOfClass` "/Game/Blueprints/Manager/BP_GameManager.BP_GameManager_C"))
              (set `GameManager.BlockPlayerMovement` true _returnvalue_5)
              (elif (and (== _array_element "wood shop") (`self.IsContact`) (`self.bIsRented`) (`self.IsShopChoiceOpen`))
                (bind _returnvalue_6 (`self.ConvertToCarpenterShop`))
                (`Widget.RemoveFromParent` _returnvalue_4)
                (bind _output_get (set `GameManager.BlockPlayerMovement` false _returnvalue_5))
                (set `self.IsShopChoiceOpen` _output_get)
                (`self.PlaySetupAudio` _returnvalue_6)
                (elif (and (== _array_element "farm shop") (`self.IsContact`) (`self.bIsRented`) (`self.IsShopChoiceOpen`) (>= (`GameManager.IslandValue` (`self.GM`)) 1450))
                  (bind _returnvalue_7 (`self.ConvertToVegetableShop`))
                  (`Widget.RemoveFromParent` _returnvalue_4)
                  (bind _output_get_2 (set `GameManager.BlockPlayerMovement` false _returnvalue_5))
                  (set `self.IsShopChoiceOpen` _output_get_2)
                  (`self.PlaySetupAudio` _returnvalue_7)
                  (elif (and (== _array_element "fish shop") (`self.IsContact`) (`self.bIsRented`) (`self.IsShopChoiceOpen`) (>= (`GameManager.IslandValue` (`self.GM`)) 2200))
                    (bind _returnvalue_8 (`self.ConvertToFishShop`))
                    (`Widget.RemoveFromParent` _returnvalue_4)
                    (bind _output_get_3 (set `GameManager.BlockPlayerMovement` false _returnvalue_5))
                    (set `self.IsShopChoiceOpen` _output_get_3)
                    (`self.PlaySetupAudio` _returnvalue_8)
                    (elif (and (== _array_element "ore shop") (`self.IsContact`) (`self.bIsRented`) (`self.IsShopChoiceOpen`) (>= (`GameManager.IslandValue` (`self.GM`)) 3000))
                      (bind _returnvalue_9 (`self.ConvertToOresShop`))
                      (`Widget.RemoveFromParent` _returnvalue_4)
                      (bind _output_get_4 (set `GameManager.BlockPlayerMovement` false _returnvalue_5))
                      (set `self.IsShopChoiceOpen` _output_get_4)
                      (`self.PlaySetupAudio` _returnvalue_9)
                      (elif (and (== _array_element "make fishing") (`self.IsContact`) (`self.bIsRented`))
                        (bind _returnvalue_10 (`self.ConvertToPond`))
                        (`self.PlaySetupAudio` _returnvalue_10)
                        (elif (and (== _array_element "make mining") (`self.IsContact`) (`self.bIsRented`))
                          (bind _returnvalue_11 (`self.ConvertToMiningLand`))
                          (`self.PlaySetupAudio` _returnvalue_11)
                          (elif (and (== _array_element "ok") (`self.IsShopChoiceOpen`))
                            (`Widget.RemoveFromParent` _returnvalue_4)
                            (set `self.IsShopChoiceOpen` false)
                            (bind _returnvalue_12 (`GameplayStatics.GetActorOfClass` "/Game/Blueprints/Manager/BP_GameManager.BP_GameManager_C"))
                            (set `GameManager.BlockPlayerMovement` false _returnvalue_12)))))))))))))))

(event `self.Overlap.OnComponentEndOverlap`
  (params (OverlappedComponent :type "PrimitiveComponent Object Reference") (OtherActor :type "Actor Object Reference") (OtherComp :type "PrimitiveComponent Object Reference") (OtherBodyIndex :type Integer))
  (if (`self.ActorHasTag` OtherActor "Player")
    (set `self.IsContact` false)
    (`SceneComponent.SetVisibility` (`self.Widget`) false false)))

(fn `PlaySetupAudio`
  (params (SoundType :type Boolean))
  (if SoundType
    (`GameplayStatics.PlaySound2D` "/Game/WAV/notification/sucess_01.sucess_01" 1.0 1.0 0.0 null null)
    (else
      (`GameplayStatics.PlaySound2D` "/Game/WAV/notification/error_01.error_01" 1.0 1.0 0.0 null null))))

(fn `SetConfirmationText`
  (params (InputName :type String))
  (returns (count :type Integer))
  (bind _returnvalue (`|CreateWidget` "/Game/UI/widgets/sample_windows/popup/WBP_Confirmation.WBP_Confirmation_C"))
  (`UserWidget.AddToViewport` _returnvalue 0)
  (set `/Game/UI/widgets/sample_windows/popup/WBP_Confirmation.SetupStrngName` InputName _returnvalue)
  (return (`/Game/UI/widgets/sample_windows/popup/WBP_Confirmation.IsConfirmedCount` _returnvalue)))

(fn `UserConstructionScript`)