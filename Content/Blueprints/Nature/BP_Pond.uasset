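; BP_Pond is a pond actor that transfers items when an actor tagged Player overlaps its Barrier component.
; After calling TransferItems, it shows the ItemsUpdatedPrompt on WBP_MainUI for a few seconds, without first checking whether items are ready.
; Every Tick, it sets its Widget component's visibility from GetAreItemsReady, so the widget appears only while items are ready.
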(event `self.Barrier.OnComponentBeginOverlap`
  (params (OverlappedComponent :type "PrimitiveComponent Object Reference") (OtherActor :type "Actor Object Reference") (OtherComp :type "PrimitiveComponent Object Reference") (OtherBodyIndex :type Integer) (bFromSweep :type Boolean) (SweepResult :type "HitResult Structure (by ref)"))
  (if (`self.ActorHasTag` OtherActor "Player")
    (`self.TransferItems`)
    (bind _foundwidgets (`WidgetBlueprintLibrary.GetAllWidgetsOfClass` "/Game/Widgets/WBP_MainUI.WBP_MainUI_C"))
    (bind _itemsupdatedprompt (`/Game/Widgets/WBP_MainUI.ItemsUpdatedPrompt` (`|GetArrayItem` _foundwidgets)))
    (`Widget.SetVisibility` _itemsupdatedprompt "Visible")
    (`KismetSystemLibrary.Delay` 5.0)
    (`Widget.SetVisibility` _itemsupdatedprompt "Hidden")))

(event `self.ReceiveTick`
  (params (DeltaSeconds :type "Float (single-precision)"))
  (bind _returnvalue (`self.GetAreItemsReady`))
  (`SceneComponent.SetVisibility` (`self.Widget`) _returnvalue false))

(fn `UserConstructionScript`)