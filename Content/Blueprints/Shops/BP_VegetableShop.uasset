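; BP_VegetableShop is a voice-controlled vegetable shop that the player operates by speaking while nearby.
; Box overlap with BP_MyPlayer sets a contact flag and binds TriggerSpeech to the speech recognition subsystem; leaving only clears the flag.
; Saying "open shop" in range shows WBP_Shop and blocks movement through BP_GameManager.
; While open, "yes" calls SellItem with a sound, and "ok" closes the widget and restores movement.
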(event `self.Box.OnComponentBeginOverlap`
  (params (OverlappedComponent :type "PrimitiveComponent Object Reference") (OtherActor :type "Actor Object Reference") (OtherComp :type "PrimitiveComponent Object Reference") (OtherBodyIndex :type Integer) (bFromSweep :type Boolean) (SweepResult :type "HitResult Structure (by ref)"))
  (bind _asbp_my_player (cast `/Game/Blueprints/Player/BP_MyPlayer` OtherActor))
  (set `self.IsContact` true)
  (add `SpeechRecognitionSubsystem.OnWordsSpoken` (subsystem `SpeechRecognitionSubsystem`) (delegate `TriggerSpeech`)))

(event `TriggerSpeech`
  (params (Text :type "RecognisedPhrases Structure"))
  (for _array_element (`.phrases` (break `RecognisedPhrases` Text))
    (if (and (== _array_element "open shop") (`self.IsContact`))
      (bind _returnvalue (`|CreateWidget` "/Game/Widgets/WBP_Shop.WBP_Shop_C"))
      (`UserWidget.AddToViewport` _returnvalue 0)
      (bind _output_get (set `self.shopISOpen` true))
      (bind _returnvalue_2 (`GameplayStatics.GetActorOfClass` "/Game/Blueprints/Manager/BP_GameManager.BP_GameManager_C"))
      (set `GameManager.BlockPlayerMovement` _output_get _returnvalue_2)
      (elif (and (== _array_element "yes") (`self.shopISOpen`))
        (`self.SellItem` (stale `self.Box.OnComponentBeginOverlap` _asbp_my_player))
        (`GameplayStatics.PlaySound2D` "/Game/AUDIO/coin_item/used_01_Cue.used_01_Cue" 1.0 1.0 0.0 null null)
        (elif (and (== _array_element "ok") (`self.shopISOpen`))
          (`Widget.RemoveFromParent` _returnvalue)
          (bind _output_get_2 (set `self.shopISOpen` false))
          (set `GameManager.BlockPlayerMovement` _output_get_2 _returnvalue_2))))))

(event `self.Box.OnComponentEndOverlap`
  (params (OverlappedComponent :type "PrimitiveComponent Object Reference") (OtherActor :type "Actor Object Reference") (OtherComp :type "PrimitiveComponent Object Reference") (OtherBodyIndex :type Integer))
  (cast `/Game/Blueprints/Player/BP_MyPlayer` OtherActor)
  (set `self.IsContact` false))

(fn `UserConstructionScript`)