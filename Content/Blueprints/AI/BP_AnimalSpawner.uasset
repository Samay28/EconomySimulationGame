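; BP_AnimalSpawner is an actor that populates the area around itself with cows when play begins.
; BeginPlay runs four spawn calls, each at its own random reachable navigation point within a fixed radius of the spawner.
; Three calls spawn BP_Cow, while the second has no class set.
; There is no respawn logic, and the construction script is empty.
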(event `self.ReceiveBeginPlay`
  (`|SpawnActorFromClass` "/Game/Blueprints/AI/Cows/BP_Cow.BP_Cow_C" (`KismetMathLibrary.MakeTransform` (`NavigationSystemV1.K2_GetRandomReachablePointInRadius` (`self.K2_GetActorLocation`) 3000.0 null null)) "Undefined" "MultiplyWithRoot" null null)
  (`|SpawnActorFromClass` "/Game/Blueprints/AI/Cows/BP_Cow.BP_Cow_C" (`KismetMathLibrary.MakeTransform` (`NavigationSystemV1.K2_GetRandomReachablePointInRadius` (`self.K2_GetActorLocation`) 3000.0 null null)) "Undefined" "MultiplyWithRoot" null null)
  (`|SpawnActorFromClass` "/Game/Blueprints/AI/Cows/BP_Cow.BP_Cow_C" (`KismetMathLibrary.MakeTransform` (`NavigationSystemV1.K2_GetRandomReachablePointInRadius` (`self.K2_GetActorLocation`) 3000.0 null null)) "Undefined" "MultiplyWithRoot" null null)
  (`|SpawnActorFromClass` "/Game/Blueprints/AI/Cows/BP_Cow.BP_Cow_C" (`KismetMathLibrary.MakeTransform` (`NavigationSystemV1.K2_GetRandomReachablePointInRadius` (`self.K2_GetActorLocation`) 3000.0 null null)) "Undefined" "MultiplyWithRoot" null null))

(fn `UserConstructionScript`)